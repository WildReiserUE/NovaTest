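; BP_StartController is the player controller for the start menu, offering start and exit actions.
; On BeginPlay it disables input, adds W_StartUI to the viewport and binds its click dispatchers, setting UI-only input only when it has to create the widget.
; Start unbinds the dispatchers, removes the widget and opens SceneMap by object reference, while Exit quits the game.
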(event Custom|ClickExit_Event_0
  (Game|QuitGame 0 "Quit" false))

(event Custom|ClickStart_Event_0
  (bind _startui (Variables|Default|GetStartUI))
  (EventDispatchers|UnbindallEventsfromClickStart _startui)
  (EventDispatchers|UnbindallEventsfromClickExit _startui)
  (Widget|RemovefromParent _startui)
  (Game|OpenLevel(byObjectReference) "/Game/NovaTest/Maps/SceneMap.SceneMap"))

(event EventBeginPlay
  (bind _self self)
  (Input|DisableInput self)
  (Utilities|IsValid (Variables|Default|GetStartUI)
    (:Is%20Valid
      (UserInterface|Viewport|AddtoViewport (Variables|Default|GetStartUI) 0)
      (EventDispatchers|AssignClickExit (Variables|Default|GetStartUI) (delegate Custom|ClickExit_Event_0))
      (EventDispatchers|AssignClickStart (Variables|Default|GetStartUI) (delegate Custom|ClickStart_Event_0)))
    (:Is%20Not%20Valid
      (bind _returnvalue (UserInterface|CreateWidget "/Game/NovaTest/UI/Start/W_StartUI.W_StartUI_C" _self))
      (bind _output_get (Variables|Default|SetStartUI _returnvalue))
      (Input|SetInputModeUIOnly _self _output_get "DoNotLock")
      (UserInterface|Viewport|AddtoViewport (Variables|Default|GetStartUI) 0)
      (EventDispatchers|AssignClickExit (Variables|Default|GetStartUI) (delegate Custom|ClickExit_Event_0))
      (EventDispatchers|AssignClickStart (Variables|Default|GetStartUI) (delegate Custom|ClickStart_Event_0)))))

(fn ConstructionScript)