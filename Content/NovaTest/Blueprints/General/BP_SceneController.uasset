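; Player controller for a preview scene that shows a BP_Preview_Static actor built around parts collected from BP_NovaInstance.
; On possessing BP_ClearPawn it shows SceneUI, spawns the preview, passes it the parts and binds Back to open StartMap.
; Holding left mouse on an active selected part spins the preview through RotatingMovement from input axes.
; Focus events move the spring arm to the part or back, with gated Tick interpolating arm length for zoom.
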(event Custom|PressBack_Event_0
  (bind _sceneui (Variables|Default|GetSceneUI))
  ;[1 1 1] Create User Interface after posses on Pawn and bind UI buttons
  (EventDispatchers|UnbindallEventsfromPressBack _sceneui)
  (Widget|RemovefromParent _sceneui)
  (Game|OpenLevel(byObjectReference) "/Game/NovaTest/Maps/StartMap.StartMap"))

(event Custom|CreatePreview
  ;[1 1 1] Spawn Prewiev Actor
  (bind _asbp_nova_instance (Utilities|Casting|CastToBP_NovaInstance (Game|GetGameInstance)))
  (bind (_bresult _parts) (Default|CollectParts _asbp_nova_instance))
  (if _bresult
    (bind _returnvalue (Game|SpawnActorfromClass "/Game/NovaTest/Blueprints/Objects/BP_Preview_Static.BP_Preview_Static_C" (Math|Transform|MakeTransform "270.000000,0.000000,220.000000" "0.000000,150.000000,90.000000" "1,1,1") "AlwaysSpawn" self 0))
    (bind _output_get (Variables|Default|SetPreviewActor _returnvalue))
    (Variables|Default|SetBaseRotation (Transformation|GetActorRotation _returnvalue))
    (Variables|Default|SetDefaultLenght (Variables|/Script/Engine.SpringArmComponent|GetTargetArmLength (Variables|/Game/NovaTest/Blueprints/Objects/BP_Preview_Static.BP_Preview_Static_C|GetSpringArm _returnvalue)))
    (Default|UpdateUI (Variables|Default|GetSceneUI) _parts _output_get)))

(event Custom|FocusCamera
  (bind _sceneui (Variables|Default|GetSceneUI))
  ;[1 1 1] SmoothFocusCamera
  (Transformation|SetWorldLocation (Variables|/Game/NovaTest/Blueprints/Objects/BP_Preview_Static.BP_Preview_Static_C|GetSpringArm (Variables|Default|GetPreviewActor)) (.Origin (Collision|GetComponentBounds (.MeshRef (Utilities|Struct|BreakS_Interact_Info (Utilities|Array|Get(acopy) (Variables|/Game/NovaTest/UI/Scene/W_SceneUI.W_SceneUI_C|GetInteract%20Info%20Array _sceneui) (Variables|/Game/NovaTest/UI/Scene/W_SceneUI.W_SceneUI_C|GetSelectedPart _sceneui)))))) false false)
  (Utilities|FlowControl|Gate true) ; enters at Open
)

(event Custom|CloseFocusForward
  ;[1 1 1] SmoothFocusCamera
  (Utilities|FlowControl|Gate true) ; enters at Close
)

(event Custom|FocusBack
  ;[1 1 1] SmoothFocusCamera
  (Transformation|SetRelativeLocation (Variables|/Game/NovaTest/Blueprints/Objects/BP_Preview_Static.BP_Preview_Static_C|GetSpringArm (Variables|Default|GetPreviewActor)) "0, 0, 0" false false)
  (Utilities|FlowControl|Gate true) ; enters at Open
)

(event Custom|CloseFocusBack
  ;[1 1 1] SmoothFocusCamera
  (Utilities|FlowControl|Gate true) ; enters at Close
)

(event EventTick
  (params (DeltaSeconds :type Float%20%28single-precision%29))
  (bind _returnvalue (Utilities|Time|GetWorldDeltaSeconds))
  (bind _returnvalue_2 (Class|Actor|GetInputAxisKeyValue))
  (bind _returnvalue_3 (Class|Actor|GetInputAxisKeyValue))
  (bind _returnvalue_4 (/ 1.0 _returnvalue))
  (bind _returnvalue_5 (* _returnvalue_2 _returnvalue_4 -1.0))
  (bind _returnvalue_6 (* _returnvalue_3 _returnvalue_4 -1.0))
  ;[1 1 1] Rotating object
  (Utilities|FlowControl|Sequence
    (:then_0
      (Utilities|FlowControl|Gate true
        (:Exit
          (Utilities|FlowControl|Sequence
            (:then_0
              (Math|Float|CompareFloat _returnvalue_2 0.0
                (:>
                  (CallFunction|RotateFunction (Variables|Default|GetPreviewActor) _returnvalue_6 _returnvalue_5 :!label _label))
                (:==
                  (if (not (or (!= _returnvalue_2 0.0) (!= _returnvalue_3 0.0)))
                    (CallFunction|RotateFunction (Variables|Default|GetPreviewActor) 0.0 0.0)))
                (:<
                  (goto _label))))
            (:then_1
              (Math|Float|CompareFloat _returnvalue_3 0.0
                (:>
                  _)
                (:<
                  _))
              (CallFunction|RotateFunction (Variables|Default|GetPreviewActor) _returnvalue_6 _returnvalue_5))))))
    (:then_1
      ;[1 1 1] SmoothFocusCamera
      (Utilities|FlowControl|Gate true
        (:Exit
          (if (Math|Float|NearlyEqual(Float) (Variables|Default|GetDefaultLenght) (Variables|Default|GetTargetLenght) 1e-06)
            (CallFunction|CloseFocusForward)
            (else
              (Variables|Default|SetTargetLenght (/ (Variables|Default|GetDefaultLenght) 1.5))
              (CallFunction|SmoothMove (Variables|Default|GetTargetLenght)))))))
    (:then_2
      (Utilities|FlowControl|Gate true
        (:Exit
          (if (Math|Float|NearlyEqual(Float) (Variables|Default|GetDefaultLenght) (Variables|Default|GetTargetLenght) 1e-06)
            (CallFunction|CloseFocusBack)
            (else
              (CallFunction|SmoothMove (Variables|Default|GetDefaultLenght)))))))))

(event EventPossess
  (params (PossessedPawn :type Pawn%20Object%20Reference))
  ;[1 1 1] Create User Interface after posses on Pawn and bind UI buttons
  (Utilities|Casting|CastToBP_ClearPawn PossessedPawn)
  (Utilities|IsValid (Variables|Default|GetSceneUI)
    (:Is%20Valid
      (UserInterface|Viewport|AddtoViewport (Variables|Default|GetSceneUI) 0))
    (:Is%20Not%20Valid
      (bind _returnvalue (UserInterface|CreateWidget "/Game/NovaTest/UI/Scene/W_SceneUI.W_SceneUI_C" self))
      (bind _output_get (Variables|Default|SetSceneUI _returnvalue))
      (UserInterface|Viewport|AddtoViewport _output_get 0)
      (Input|SetInputModeGameandUI self (Variables|Default|GetSceneUI) "DoNotLock" true)))
  (EventDispatchers|AssignPressBack (Variables|Default|GetSceneUI) (delegate Custom|PressBack_Event_0))
  (CallFunction|CreatePreview))

(event Input|MouseEvents|LeftMouseButton
  (params (Key :type Key%20Structure :default "None"))
  (bind _returnvalue (Utilities|Time|GetWorldDeltaSeconds))
  (bind _returnvalue_2 (Class|Actor|GetInputAxisKeyValue))
  (bind _returnvalue_3 (Class|Actor|GetInputAxisKeyValue))
  (bind _sceneui (Variables|Default|GetSceneUI))
  (bind _returnvalue_4 (/ 1.0 _returnvalue))
  (bind _interact_info_array (Variables|/Game/NovaTest/UI/Scene/W_SceneUI.W_SceneUI_C|GetInteract%20Info%20Array _sceneui))
  (bind _selectedpart (Variables|/Game/NovaTest/UI/Scene/W_SceneUI.W_SceneUI_C|GetSelectedPart _sceneui))
  (bind _returnvalue_5 (* _returnvalue_2 _returnvalue_4 -1.0))
  (bind _returnvalue_6 (* _returnvalue_3 _returnvalue_4 -1.0))
  (bind _output (Utilities|Array|Get(acopy) _interact_info_array _selectedpart))
  (bind (_meshref _bisactive) (Utilities|Struct|BreakS_Interact_Info _output))
  ;[1 1 1] Rotating object
  (:Pressed
    (if _bisactive
      (Variables|Default|SetMesh%20Ref _meshref)
      (Utilities|FlowControl|Gate true) ; enters at Open
    ))
  (:Released
    (Variables|/Script/Engine.RotatingMovementComponent|SetRotationRate (Variables|/Game/NovaTest/Blueprints/Objects/BP_Preview_Static.BP_Preview_Static_C|GetRotatingMovement (Variables|Default|GetPreviewActor)) "0, 0, 0")
    (Utilities|FlowControl|Gate true) ; enters at Close
  ))

(fn ConstructionScript)

(fn RotateFunction
  (params (ActorRef :type BP%20Preview%20Static%20Object%20Reference) (Rotation%20Rate%20X%20%28Roll%29 :type Float%20%28single-precision%29) (Rotation%20Rate%20Y%20%28Pitch%29 :type Float%20%28single-precision%29))
  (Variables|/Script/Engine.RotatingMovementComponent|SetRotationRate (Variables|/Game/NovaTest/Blueprints/Objects/BP_Preview_Static.BP_Preview_Static_C|GetRotatingMovement ActorRef) (Math|Rotator|MakeRotator Rotation%20Rate%20X%20%28Roll%29 Rotation%20Rate%20Y%20%28Pitch%29 0.0))
  (return))

(fn SmoothMove
  (params (Target :type Float%20%28single-precision%29))
  (bind _previewactor (Variables|Default|GetPreviewActor))
  (bind _springarm (Variables|/Game/NovaTest/Blueprints/Objects/BP_Preview_Static.BP_Preview_Static_C|GetSpringArm _previewactor))
  (Variables|/Script/Engine.SpringArmComponent|SetTargetArmLength _springarm (Math|Interpolation|FInterpTo (Variables|/Script/Engine.SpringArmComponent|GetTargetArmLength _springarm) Target (Utilities|Time|GetWorldDeltaSeconds) 3.0)))