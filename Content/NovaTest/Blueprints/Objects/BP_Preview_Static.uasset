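; BP_Preview_Static is a preview actor that builds its display from static mesh components added at runtime.
; AddSomeMesh creates a shadowless component for a valid mesh, snaps it to RotationSphere and records it as an inactive entry in InteractInfoArray.
; It returns the attach result and the updated array, or failure for an invalid mesh; the construction script is empty.
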(fn ConstructionScript)

(fn AddSomeMesh
  (params (NewMesh :type Static%20Mesh%20Object%20Reference))
  (Utilities|IsValid NewMesh
    (:Is%20Valid
      (bind _returnvalue (AddComponent|AddStaticMeshComponent false (Math|Transform|MakeTransform "0, 0, 0" (Transformation|GetActorRotation) "1,1,1")))
      (Rendering|SetCastShadow _returnvalue false)
      (Utilities|Array|Add (Variables|Default|GetInteractInfoArray) (Utilities|Struct|MakeS_Interact_Info _returnvalue false))
      (Components|StaticMesh|SetStaticMesh _returnvalue NewMesh)
      (bind _returnvalue_2 (Transformation|AttachComponentToComponent _returnvalue (Variables|Default|GetRotationSphere) "None" "SnapToTarget" "SnapToTarget" "SnapToTarget" false))
      (return _returnvalue_2 (Variables|Default|GetInteractInfoArray)))
    (:Is%20Not%20Valid
      (return false 0))))